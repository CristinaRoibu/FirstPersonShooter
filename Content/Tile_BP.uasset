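; Tile_BP is one segment of an endlessly spawned level, populated on BeginPlay with containers, sacks and AI characters.
; A pawn-blocking wall starts locked, unlocks while the first-person player overlaps the trigger box, and relocks on exit.
; After a short delay, entry destroys the fifth-from-last tile and its props, then asks TileGameMode to spawn another.
; GetAttachLoc exposes the Arrow transform as an attach point.
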(event OnComponentEndOverlap(BoxCollision)
  (params (OverlappedComponent :type Primitive%20Component%20Object%20Reference) (OtherActor :type Actor%20Object%20Reference) (OtherComp :type Primitive%20Component%20Object%20Reference) (OtherBodyIndex :type Integer))
  (Utilities|Casting|CastToFirstPersonCharacter OtherActor)
  (CallFunction|LockWall))

(event OnComponentBeginOverlap(BoxCollision)
  (params (OverlappedComponent :type Primitive%20Component%20Object%20Reference) (OtherActor :type Actor%20Object%20Reference) (OtherComp :type Primitive%20Component%20Object%20Reference) (OtherBodyIndex :type Integer) (bFromSweep :type Boolean) (SweepResult :type Hit%20Result%20Structure%20%28by%20ref%29))
  (Utilities|Casting|CastToFirstPersonCharacter OtherActor)
  (CallFunction|UnlockWall)
  (bind _astile_game_mode (Utilities|Casting|CastToTileGameMode (Game|GetGameMode)))
  (Utilities|FlowControl|Delay 1.5)
  (CallFunction|DestroyTile)
  (Default|SpawnTile _astile_game_mode))

(event Custom|DestroyTile
  ;[1 1 1] destroy the tile you just left
  (bind _astile_game_mode (Utilities|Casting|CastToTileGameMode (Game|GetGameMode)))
  (if (not (<= (- (Utilities|Array|Length (Variables|/Game/TileGameMode.TileGameMode_C|GetTiles _astile_game_mode)) 5) -1))
    (bind _astile_bp (Utilities|Casting|CastToTile_BP (Utilities|Array|Get(acopy) (Variables|/Game/TileGameMode.TileGameMode_C|GetTiles _astile_game_mode) (- (Utilities|Array|Length (Variables|/Game/TileGameMode.TileGameMode_C|GetTiles _astile_game_mode)) 5))))
    (for _array_element (Variables|/Script/PewPew.Tile|GetPropsToDelete _astile_bp)
      (Actor|DestroyActor _array_element))
    (Actor|DestroyActor _astile_bp)))

(event EventBeginPlay
  (CallFunction|LockWall)
  (Class|Tile|PlaceActors "/Game/PROPS/Container_Blueprint.Container_Blueprint_C")
  (Class|Tile|PlaceAI "/Game/TRAsh/ThirdPersonCharacter.ThirdPersonCharacter_C")
  (Class|Tile|PlaceActors "/Game/PROPS/Container_Blueprint.Container_Blueprint_C")
  (Class|Tile|PlaceActors "/Game/PROPS/Sack1_Blueprint.Sack1_Blueprint_C"))

(fn ConstructionScript)

(fn GetAttachLoc
  (return (Transformation|GetWorldTransform (Variables|Default|GetArrow))))

(fn LockWall
  (Collision|SetCollisionResponsetoChannel (Variables|Default|GetWallBlock) "ECC_Pawn" "ECR_Block"))

(fn UnlockWall
  (Collision|SetCollisionResponsetoChannel (Variables|Default|GetWallBlock) "ECC_Pawn" "ECR_Ignore"))