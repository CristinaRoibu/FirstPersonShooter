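; AI controller for guard NPCs that runs the GuardBehaviour behavior tree on possession and plays a death animation on unpossess.
; Perception updates for a non-"Enemy" first-person player toggle the pawn's shooting flag and write either the focus target or last seen location to the blackboard.
; Tick polls the pawn's Attacked flag, sets the player controller as focus, then clears the flag after a short delay.
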(event OnTargetPerceptionUpdated(AIPerception)
  (params (Actor :type Actor%20Object%20Reference) (Stimulus :type AI%20Stimulus%20Structure))
  (bind (_age _expirationage _strength _stimuluslocation _receiverlocation _tag _bsuccessfullysensed) (Utilities|Struct|BreakAIStimulus Stimulus))
  (bind _bbcomp (Variables|Default|GetBbComp))
  (bind _newfocus (Variables|Default|GetNewFocus))
  ;[1 1 1] if target is an enemy like you dont shoot
  (if (not (Actor|ActorHasTag Actor "Enemy"))
    (Utilities|Casting|CastToFirstPersonCharacter Actor)
    (bind _asthird_person_character (Utilities|Casting|CastToThirdPersonCharacter (Pawn|GetControlledPawn)))
    (Variables|/Game/TRAsh/ThirdPersonCharacter.ThirdPersonCharacter_C|SetShootin _asthird_person_character _bsuccessfullysensed)
    (if _bsuccessfullysensed
      (AI|Components|Blackboard|SetValueasObject _bbcomp _newfocus Actor)
      (AI|Components|Blackboard|ClearValue (Variables|Default|GetBbComp) (Utilities|Name|MakeLiteralName "LastSeenLocation"))
      (else
        (AI|Components|Blackboard|ClearValue _bbcomp _newfocus)
        (AI|Components|Blackboard|SetValueasVector (Variables|Default|GetBbComp) (Utilities|Name|MakeLiteralName "LastSeenLocation") _stimuluslocation)))))

(event EventTick
  (params (DeltaSeconds :type Float%20%28single-precision%29))
  (bind _aipawn (Variables|Default|GetAIPawn))
  ;[1 1 1] Check if the enemy is being attacked by the player__BUG None trying to read AIPawn
  (if (Variables|/Script/PewPew.MeinCharacter|GetAttacked _aipawn)
    (AI|Components|Blackboard|SetValueasObject (Variables|Default|GetBbComp) (Variables|Default|GetNewFocus) (Game|GetPlayerController 0))
    (Utilities|FlowControl|Delay 0.025)
    (Variables|/Script/PewPew.MeinCharacter|SetAttacked _aipawn false)))

(event EventOnUnpossess
  (params (UnpossessedPawn :type Pawn%20Object%20Reference))
  (bind _asthird_person_character (Utilities|Casting|CastToThirdPersonCharacter UnpossessedPawn))
  (Components|Animation|PlayAnimation (Variables|/Script/Engine.Character|GetMesh _asthird_person_character) "/Game/AnimStarterPack/Death_1.Death_1" false)
  (|CallParentFunction UnpossessedPawn))

(event EventOnPossess
  (params (PossessedPawn :type Pawn%20Object%20Reference))
  (bind _blackboardcomponent (Class|AIController|UseBlackboard "/Game/PatrolData.PatrolData"))
  (AI|RunBehaviorTree "/Game/GuardBehaviour.GuardBehaviour")
  (bind _output_get (Variables|Default|SetBbComp _blackboardcomponent))
  (AI|Components|Blackboard|SetValueasBool _output_get (Utilities|Name|MakeLiteralName "CanSetLastSennKey") true)
  ;[1 1 1] set AIPawn ref
  (bind _asthird_person_character (Utilities|Casting|CastToThirdPersonCharacter (Pawn|GetControlledPawn)))
  (Variables|Default|SetAIPawn _asthird_person_character))

(fn ConstructionScript)

(fn GetWaypointfromArray
  (bind _asthird_person_character (Utilities|Casting|CastToThirdPersonCharacter (Pawn|GetControlledPawn)))
  (return (Utilities|Array|Get(acopy) (Variables|/Game/TRAsh/ThirdPersonCharacter.ThirdPersonCharacter_C|GetPatrolPoints_0 _asthird_person_character)) (Utilities|Name|MakeLiteralName "WayPoint")))